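; Game instance Blueprint that reports Epic Online Services and Oculus Platform initialization through debug messages.
; When the Oculus subsystem start event fires, it requests the logged-in user regardless of success, then starts the message pump and checks entitlement.
; User details and entitlement results are only printed or logged, with no enforcement on failure.
; The EOS handler just prints readiness, and the EOS Setup function is an empty stub.
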(event Custom|OvrPlatformSubsystemStarted
  (params (OvrPlatformReady :type Boolean))
  (Development|PrintString (Utilities|String|SelectString "JJJ: OVR Initialzed" "JJJ: OVR  FAILED" OvrPlatformReady))
  (bind (_user _errormsg) (Class|OvrRequestsBlueprintLibrary|UserGetLoggedinUser)
    (:Then
      (Class|OvrPlatformSubsystem|StartMessagePump (Subsystems|GetOvrPlatformSubsystem))
      (bind _errormsg_2 (Class|OvrRequestsBlueprintLibrary|EntitlementGetIsViewerEntitled)
        (:Success
          (Development|PrintString "JJJ: PASSED ENTITLEMENT"))
        (:Failure
          (Development|PrintString _errormsg_2))))
    (:Success
      (Development|PrintString "JJJ: GET USER OKAY")
      (Development|PrintString (Class|OvrPlatformUtilsLibrary|ToString(OvrId) (.ID (Utilities|Struct|BreakOvrUser _user))))
      (Development|PrintString (.OculusID (Utilities|Struct|BreakOvrUser _user)))
      (Utilities|String|LogString (.DisplayName (Utilities|Struct|BreakOvrUser _user))))
    (:Failure
      (Development|PrintString "JJJ: GET USER FAILED")
      (Development|PrintString _errormsg))))

(event Custom|EOSInitialized
  (params (EOS%20Ready :type Boolean))
  (if EOS%20Ready
    (Development|PrintString "JJJ: EOS Initialized")
    (else
      (Development|PrintString "JJJ: EOS FAILED"))))

(fn EOSSetup)